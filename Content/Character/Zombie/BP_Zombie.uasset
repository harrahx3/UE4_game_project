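; BP_Zombie is an enemy zombie character with custom events for patrolling, chasing and firing at the player.
; Firing loops a timer that line-traces toward the player and subtracts life from BP_Akai.
; Patrol repeats random-point moves, Poursuite runs faster to the player's position, and a one-second timer ends pursuit after a few ticks, resuming patrol.
; BeginPlay and PawnSensing handlers are empty, with earlier behavior-tree and sensing experiments left disconnected.
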(event `self.ReceiveBeginPlay`
  ;[1 1 1] Maniere alternative de gerer le behaviour tree plutot que le BP_AIController
)

(event `Start Firing`
  ;[1 1 1] Fire
  (`KismetSystemLibrary.K2_SetTimer` null "Fire Weapon" (`self.AI_fireRate`) true))

(event `Fire Weapon`
  ;[1 1 1] Fire
  (bind (_outhit _returnvalue) (`KismetSystemLibrary.LineTraceSingle` :`Start` (`self.K2_GetActorLocation`) :`End` (`self.K2_GetActorLocation` (`GameplayStatics.GetPlayerCharacter` 0)) :`TraceChannel` "TraceTypeQuery1" :`DrawDebugType` "ForDuration"))
  (if _returnvalue
    (bind _asbp_akai (cast `/Game/Character/Akai/BP_Akai` (`.HitActor` (`GameplayStatics.BreakHitResult` _outhit))))
    (`/Game/Character/Akai/BP_Akai.addLife` _asbp_akai (* (`self.FireDamage`) -1.0))))

(event `Stop Firing`
  ;[1 1 1] Fire
  (`KismetSystemLibrary.K2_ClearTimer` null "Fire Weapon"))

(event `self.PawnSensing.OnSeePawn`
  (params (Pawn :type "Pawn Object Reference"))
  ;[1 1 1] PawnSensing
)

(event `self.PawnSensing.OnHearNoise`
  (params (Instigator :type "Pawn Object Reference") (Location :type "Vector Structure (by ref)") (Volume :type "Float (single-precision)"))
  ;[1 1 1] PawnSensing
)

(event `Patrol`
  ;[1 1 1] AI Patrol and follow
  (set `CharacterMovementComponent.MaxWalkSpeed` 180.0 (`self.CharacterMovement`))
  (`|AIMoveTo` self (`NavigationSystem.K2_GetRandomReachablePointInRadius` (`self.K2_GetActorLocation`) 5000.0)
    (:`OnSuccess`
      (`self.Patrol`))))

(event `ResetTimer`
  ;[1 1 1] AI Patrol and follow
  ;;[1 1 1] Ajouter evenement OnSeePawn
  (`/Engine/EditorBlueprintResources/StandardMacros.DoOnce` false :!via `Reset`
    (:`Completed`
      (`self.Timer`))))

(event `Poursuite`
  ;[1 1 1] AI Patrol and follow
  (set `CharacterMovementComponent.MaxWalkSpeed` 300.0 (`self.CharacterMovement`))
  (`|AIMoveTo` self (`self.K2_GetActorLocation` (`GameplayStatics.GetPlayerCharacter` 0))))

(event `Timer`
  ;[1 1 1] AI Patrol and follow
  (set `self.Time` 0.0)
  (bind _returnvalue (`KismetSystemLibrary.K2_SetTimerDelegate` (delegate `DureePoursuite`) 1.0 true))
  (set `self.TimerRef` _returnvalue))

(event `DureePoursuite`
  ;[1 1 1] AI Patrol and follow
  (if (<= (`self.Time`) 3.0)
    (set `self.Time` (+ (`self.Time`) 1.0))
    (else
      (`KismetSystemLibrary.K2_ClearAndInvalidateTimerHandle` (`self.TimerRef`))
      (`MovementComponent.StopMovementImmediately` (`self.CharacterMovement`))
      (`self.Patrol`)
      (`self.ResetTimer`))))

(fn `UserConstructionScript`)