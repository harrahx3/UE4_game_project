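; BP_Lift is a lift actor that moves between a start and an end location as soon as play begins.
; BeginPlay stores the Platform component's world location as StartLocation, then plays a timeline.
; Each update linearly interpolates toward EndLocation by the timeline value and sets the whole actor's relative location, without sweep.
; No overlap trigger or Tick logic drives it.
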(event `self.ReceiveBeginPlay`
  (bind _startlocation (`self.startLocation`))
  (set `self.startLocation` (`SceneComponent.K2_GetComponentLocation` (`self.Platform`)))
  (bind (_direction _value) (`Timeline|Timeline_0`)
    (:`Update`
      (`self.K2_SetActorRelativeLocation` (+ (* (- (`self.endLocation`) _startlocation) _value) _startlocation)))))

(event `self.ReceiveTick`
  (params (DeltaSeconds :type "Float (single-precision)")))

(fn `UserConstructionScript`)