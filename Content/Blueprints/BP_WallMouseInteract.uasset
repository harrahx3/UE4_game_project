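; Wall actor with Rise and Down events meant to move it vertically.
; Rise plays a timeline that lerps the actor's current Z toward MaxHeight, while Down reverses the same timeline.
; The lerp starts from the live position rather than a stored origin, so reversing does not restore the starting height.
; Cursor-trace triggering and BP_Akai input toggling are disconnected, so nothing here calls either event.
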(event `Key|RightMouseButton`
  (params (Key :type "Key Structure" :default "AnyKey")))

(event `self.ReceiveActorBeginOverlap`
  (params (OtherActor :type "Actor Object Reference"))
  ;[1 1 1] Overlap
)

(event `self.ReceiveActorEndOverlap`
  (params (OtherActor :type "Actor Object Reference"))
  ;[1 1 1] Overlap
)

(event `Rise`
  (bind (_returnvalue_x _returnvalue_y _returnvalue_z) (`KismetMathLibrary.BreakVector` (`self.K2_GetActorLocation`)))
  ;[1 1 1] Rise
  (bind (_direction _z) (`Timeline|Timeline_0` :!via `PlayFromStart` :!label _label)
    (:`Update`
      (`KismetSystemLibrary.PrintString` "move")
      (`self.K2_SetActorLocation` (`KismetMathLibrary.MakeVector` _returnvalue_x _returnvalue_y (`KismetMathLibrary.Lerp` _returnvalue_z (`self.maxHeight`) _z))))))

(event `Down`
  ;[1 1 1] Rise
  (goto _label :!via `ReverseFromEnd`))

(event `self.ReceiveTick`
  (params (DeltaSeconds :type "Float (single-precision)")))

(event `self.Cube.OnComponentBeginOverlap`
  (params (OverlappedComponent :type "PrimitiveComponent Object Reference") (OtherActor :type "Actor Object Reference") (OtherComp :type "PrimitiveComponent Object Reference") (OtherBodyIndex :type Integer) (bFromSweep :type Boolean) (SweepResult :type "HitResult Structure (by ref)")))

(event `self.ReceiveBeginPlay`)

(fn `UserConstructionScript`)