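; Weapon actor that the BP_Akai player can pick up and fire.
; Overlapping its Box stores the player and enables input on the weapon; the action input then sets the player's Weapon child actor to this weapon's class.
; Leaving the Box disables input on the character rather than on the weapon.
; Shoot spawns a Bullet_BP at the Sphere's transform, passing initial and max speed.
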(event `InputAction|action`
  (params (Key :type "Key Structure"))
  (:`Pressed`
    (`ChildActorComponent.SetChildActorClass` (`/Game/Character/Akai/BP_Akai.Weapon` (`self.player_ref`)) (`GameplayStatics.GetObjectClass` self))))

(event `self.Box.OnComponentBeginOverlap`
  (params (OverlappedComponent :type "PrimitiveComponent Object Reference") (OtherActor :type "Actor Object Reference") (OtherComp :type "PrimitiveComponent Object Reference") (OtherBodyIndex :type Integer) (bFromSweep :type Boolean) (SweepResult :type "HitResult Structure (by ref)"))
  (bind _asbp_akai (cast `/Game/Character/Akai/BP_Akai` OtherActor))
  (set `self.player_ref` _asbp_akai)
  (`self.EnableInput` (`GameplayStatics.GetPlayerController` 0)))

(event `self.Box.OnComponentEndOverlap`
  (params (OverlappedComponent :type "PrimitiveComponent Object Reference") (OtherActor :type "Actor Object Reference") (OtherComp :type "PrimitiveComponent Object Reference") (OtherBodyIndex :type Integer))
  (bind _asbp_akai (cast `/Game/Character/Akai/BP_Akai` OtherActor))
  (`self.DisableInput` _asbp_akai (`GameplayStatics.GetPlayerController` 0)))

(fn `Shoot`
  (`|SpawnActorFromClass` "/Game/Blueprints/Weapons/Bullet_BP.Bullet_BP_C" (`SceneComponent.K2_GetComponentToWorld` (`self.Sphere`)) "Undefined" "OverrideRootScale" null (`self.Initial_Speed`) (`self.Max_Speed`) null))

(fn `UserConstructionScript`)