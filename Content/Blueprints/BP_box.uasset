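; BP_box is a hazard volume that deals damage over time to the BP_Akai character when it enters the Box component.
; Overlap removes Degats life immediately through a negated AddLife call, then starts a looping one-second timer.
; Each tick repeats the damage until Counter reaches Duree, then clears the timer.
; Counter is never reset, so once it is used up, later overlaps deal only the immediate hit.
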(event `self.Box.OnComponentBeginOverlap`
  (params (OverlappedComponent :type "PrimitiveComponent Object Reference") (OtherActor :type "Actor Object Reference") (OtherComp :type "PrimitiveComponent Object Reference") (OtherBodyIndex :type Integer) (bFromSweep :type Boolean) (SweepResult :type "HitResult Structure (by ref)"))
  (bind _asbp_akai (cast `/Game/Character/Akai/BP_Akai` OtherActor))
  (`/Game/Character/Akai/BP_Akai.addLife` _asbp_akai (* (`self.degats`) -1.0))
  (`self.degat`))

(event `degat`
  (bind _returnvalue (`KismetSystemLibrary.K2_SetTimerDelegate` (delegate `InfligerDegat`) 1.0 true)))

(event `InfligerDegat`
  (bind _counter (`self.counter`))
  (if (< _counter (`self.duree`))
    (`/Engine/EditorBlueprintResources/StandardMacros.IncrementInt` _counter
      (:`  `
        (`/Game/Character/Akai/BP_Akai.addLife` (stale `self.Box.OnComponentBeginOverlap` _asbp_akai) (* (`self.degats`) -1.0))))
    (else
      (`KismetSystemLibrary.K2_ClearAndInvalidateTimerHandle` (stale `degat` _returnvalue)))))

(fn `UserConstructionScript`)