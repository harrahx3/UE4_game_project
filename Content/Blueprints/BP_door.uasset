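; BP_door is an interactive hinged door that the player opens and closes with an action input, enabled only while BP_Akai overlaps it.
; An overlap check on BoxA picks one of two yaw timelines relative to the door's starting rotation, and closing reverses the active one.
; Opening and closing sounds play, and each timeline update emits noise through a PawnNoiseEmitter.
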(event `self.ReceiveBeginPlay`
  ;[1 1 1] Rotation0
  (set `self.rotation0` (`SceneComponent.RelativeRotation` (`self.door`))))

(event `self.ReceiveActorBeginOverlap`
  (params (OtherActor :type "Actor Object Reference"))
  ;[1 1 1] Overlap
  (cast `/Game/Character/Akai/BP_Akai` OtherActor)
  (`self.EnableInput` (`GameplayStatics.GetPlayerController` 0)))

(event `self.ReceiveActorEndOverlap`
  (params (OtherActor :type "Actor Object Reference"))
  ;[1 1 1] Overlap
  (cast `/Game/Character/Akai/BP_Akai` OtherActor)
  (`self.DisableInput` (`GameplayStatics.GetPlayerController` 0)))

(event `InputAction|action`
  (params (Key :type "Key Structure" :default "AnyKey"))
  ;[1 1 1] Open and close door
  (:`Pressed`
    (switch `/Game/Blueprints/enum_doorState` (`self.door state`)
      (:`NewEnumerator0`
        (`GameplayStatics.PlaySoundAtLocation` "/Game/Sounds/S_openingDoor.S_openingDoor" (`self.K2_GetActorLocation`))
        (if (`PrimitiveComponent.IsOverlappingActor` (`self.Box A`) (`GameplayStatics.GetPlayerCharacter` 0))
          (set `self.door state` "NewEnumerator1")
          (bind (_direction _rotation) (`Timeline|Timeline_door_A` :!label _label)
            (:`Update`
              (`SceneComponent.K2_SetRelativeRotation` (`self.door`) (`KismetMathLibrary.MakeRotator` (.roll (`self.rotation0`)) (.pitch (`self.rotation0`)) (+ _rotation (.yaw (`self.rotation0`)))) false false)
              (`self.Noise`))
            (:`Finished`
              (if (`|EnumEquality` (`self.door state`) "NewEnumerator0") :!label _label_2
                (`GameplayStatics.PlaySoundAtLocation` "/Game/Sounds/S_closingDoor.S_closingDoor" (`self.K2_GetActorLocation`)))))
          (else
            (set `self.door state` "NewEnumerator2")
            (bind (_direction_2 _rotation_2) (`Timeline|Timeline_door_B` :!label _label_3)
              (:`Update`
                (`SceneComponent.K2_SetRelativeRotation` (`self.door`) (`KismetMathLibrary.MakeRotator` (.roll (`self.rotation0`)) (.pitch (`self.rotation0`)) (+ _rotation_2 (.yaw (`self.rotation0`)))) false false)
                (`self.Noise`))
              (:`Finished`
                (goto _label_2))))))
      (:`NewEnumerator1`
        (set `self.door state` "NewEnumerator0")
        (goto _label :!via `Reverse`))
      (:`NewEnumerator2`
        (set `self.door state` "NewEnumerator0")
        (goto _label_3 :!via `Reverse`)))))

(fn `Noise`
  (`PawnNoiseEmitterComponent.MakeNoise` (`self.PawnNoiseEmitter`) self 1.0 (`self.K2_GetActorLocation`)))

(fn `UserConstructionScript`)