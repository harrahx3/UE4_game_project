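; BP_Window is an interactive window that the BP_Akai character can swing open and closed.
; Overlapping its Box enables input on the actor for player 0, and ending the actor overlap disables it.
; The action input drives a FlipFlop that plays or reverses a timeline, adding yaw to the GlassWindow's starting rotation.
; An opening sound plays as the motion starts, and a closing sound plays when the reverse finishes.
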(event `self.ReceiveBeginPlay`
  ;[1 1 1] Rotation0
  (set `self.rotation0` (`SceneComponent.RelativeRotation` (`self.Glass_Window`))))

(event `self.Box.OnComponentBeginOverlap`
  (params (OverlappedComponent :type "PrimitiveComponent Object Reference") (OtherActor :type "Actor Object Reference") (OtherComp :type "PrimitiveComponent Object Reference") (OtherBodyIndex :type Integer) (bFromSweep :type Boolean) (SweepResult :type "HitResult Structure (by ref)"))
  ;[1 1 1] Overlap
  (cast `/Game/Character/Akai/BP_Akai` OtherActor)
  (`self.EnableInput` (`GameplayStatics.GetPlayerController` 0)))

(event `InputAction|action`
  (params (Key :type "Key Structure" :default "AnyKey"))
  ;[1 1 1] Open door
  (:`Pressed`
    (bind _isa (`/Engine/EditorBlueprintResources/StandardMacros.FlipFlop`)
      (:`A`
        (`GameplayStatics.PlaySoundAtLocation` "/Game/Sounds/S_openingDoor.S_openingDoor" (`self.K2_GetActorLocation`))
        (bind (_direction _rotation) (`Timeline|Timeline_0` :!label _label)
          (:`Update`
            (`SceneComponent.K2_SetRelativeRotation` (`self.Glass_Window`) (`KismetMathLibrary.MakeRotator` (.roll (`self.rotation0`)) (.pitch (`self.rotation0`)) (+ _rotation (.yaw (`self.rotation0`)))) false false))
          (:`Finished`
            (if (not _isa)
              (`GameplayStatics.PlaySoundAtLocation` "/Game/Sounds/S_closingDoor.S_closingDoor" (`self.K2_GetActorLocation`))))))
      (:`B`
        (goto _label :!via `Reverse`)))))

(event `self.ReceiveActorEndOverlap`
  (params (OtherActor :type "Actor Object Reference"))
  ;[1 1 1] Overlap
  (cast `/Game/Character/Akai/BP_Akai` OtherActor)
  (`self.DisableInput` (`GameplayStatics.GetPlayerController` 0)))

(fn `UserConstructionScript`)